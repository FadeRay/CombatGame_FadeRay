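; Test weapon Blueprint that adds combo-dependent launch reactions when the player's hits land on an enemy.
; Trace and range hit events branch on whether the enemy is airborne, then on the player's ComboState, with only the first combo state wired in two branches.
; Trace hits knock airborne enemies back and down, while range hits pop grounded enemies up and apply AIrDelay to both characters.
; Construction attaches the HitBox to the Cube.
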(event `self.TraceHit_DoSomething`
  (params (Enemy :type "/Game/ThirdPersonBP/Blueprints/EnemyCharacter Object Reference"))
  (bind _combostate (`/Game/DynamicSwordAnimset/Combat_AnimBP.ComboState` (`/Game/ThirdPersonBP/Blueprints/ThirdPersonCharacter.GetAnimIns` (`self.Player`))))
  (bind _inair (`self.CheckInAir` Enemy))
  (if _inair
    (switch `int` _combostate
      (:`1`
        (set `/Game/DynamicSwordAnimset/Combat_AnimBP.BisAirInjued` true (`/Game/ThirdPersonBP/Blueprints/EnemyCharacter.GetAnimIns` Enemy))
        (`Character.LaunchCharacter` Enemy (+ (* (`self.GetActorForwardVector` Enemy) -1500.0) (0.0 0.0 -500.0)) true true)))
    (else
      (switch `int` _combostate))))

(event `self.RangeHit_DoSomething`
  (params (Enemy :type "/Game/ThirdPersonBP/Blueprints/EnemyCharacter Object Reference"))
  (bind _player (`self.Player`))
  (bind _combostate (`/Game/DynamicSwordAnimset/Combat_AnimBP.ComboState` (`/Game/ThirdPersonBP/Blueprints/ThirdPersonCharacter.GetAnimIns` _player)))
  (bind _inair (`self.CheckInAir` Enemy))
  (if _inair
    (switch `int` _combostate)
    (else
      (switch `int` _combostate
        (:`1`
          (`Character.LaunchCharacter` Enemy (`KismetMathLibrary.MakeVector` 0.0 0.0 900.0) true true)
          (`self.AIrDelay` (`Character.CharacterMovement` _player) 0.1)
          (`self.AIrDelay` (`Character.CharacterMovement` Enemy) 0.1))))))

(fn `UserConstructionScript`
  (`parent.UserConstructionScript`)
  (`SceneComponent.K2_AttachToComponent` (`self.HitBox`) (`self.Cube`) "None" "KeepWorld" "KeepWorld" "KeepWorld" true))