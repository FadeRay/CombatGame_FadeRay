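; Sword weapon Blueprint that adds launch and air-juggle reactions when its trace hits an enemy.
; The hit event checks whether the enemy is airborne and reads the player's combo state from the anim instance.
; Airborne enemies get a small or large upward launch plus a brief air delay on both characters' movement, while grounded enemies are launched high only on the third combo state.
; The construction script attaches the hit box to the sword.
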(event `self.TraceHit_DoSomething`
  (params (Enemy :type "/Game/ThirdPersonBP/Blueprints/EnemyCharacter Object Reference"))
  (bind _player (`self.Player`))
  (bind _combostate (`/Game/DynamicSwordAnimset/Combat_AnimBP.ComboState` (`/Game/ThirdPersonBP/Blueprints/ThirdPersonCharacter.GetAnimIns` _player)))
  (bind _inair (`self.CheckInAir` Enemy))
  (if _inair
    (switch `int` _combostate
      (:`0`
        (`Character.LaunchCharacter` Enemy (`KismetMathLibrary.MakeVector` 0.0 0.0 140.0) true true :!label _label))
      (:`1`
        (goto _label))
      (:`2`
        (`Character.LaunchCharacter` Enemy (`KismetMathLibrary.MakeVector` 0.0 0.0 880.0) true true :!label _label_2)))
    (else
      (switch `int` _combostate
        (:`2`
          (goto _label_2)))))
  (`self.AIrDelay` (`Character.CharacterMovement` _player) 0.1)
  (`self.AIrDelay` (`Character.CharacterMovement` Enemy) 0.1))

(fn `UserConstructionScript`
  (`parent.UserConstructionScript`)
  (`SceneComponent.K2_AttachToComponent` (`self.HitBox`) (`self.Sword`) "None" "KeepWorld" "KeepWorld" "KeepWorld" true))